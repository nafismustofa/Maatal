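; BP_Spider is an enemy spider that chases the player and can be killed by damage.
; Its PawnSensing component triggers an AI move toward player zero whenever it sees a pawn while alive.
; Damage reduces CurrentHP, which the construction script initializes from MaxHP; at zero it plays a death montage and destroys itself when the montage starts blending out.
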(event OnSeePawn(PawnSensing)
  (params (Pawn :type Pawn%20Object%20Reference))
  (if (Variables|Default|GetIsAlive)
    (AI|AIMoveTo self "0, 0, 0" (Game|GetPlayerCharacter 0) 5.0 false)))

(event Game|Damage|EventAnyDamage
  (params (Damage :type Float%20%28single-precision%29) (DamageType :type Damage%20Type%20Object%20Reference) (InstigatedBy :type Controller%20Object%20Reference) (DamageCauser :type Actor%20Object%20Reference))
  (if (Variables|Default|GetIsAlive)
    (bind _output_get (Variables|Default|SetCurrentHP (- (Variables|Default|GetCurrentHP) Damage)))
    (if (<= _output_get 0.0)
      (Variables|Default|SetIsAlive false)
      (Animation|Montage|PlayMontage (Variables|Character|GetMesh) "/Game/Animations/SpiderAnimations/AM_Spider_Death.AM_Spider_Death"
        (:OnBlendOut
          (Actor|DestroyActor))))))

(fn ConstructionScript
  (Variables|Default|SetCurrentHP (Variables|Default|GetMaxHP)))