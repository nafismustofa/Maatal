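; BP_EnemySpawner periodically spawns BP_Enemy_Spider pawns at random reachable navmesh points around itself, up to a maximum live count.
; A looping timer calls SpawnEnemy, which recursively retries when its random point lies too close to the player.
; The random-point node is pure, so the spawn location is rolled separately from the distance-checked one.
; Each spider receives a default controller and decrements the count through a bound death event.
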(event Custom|Spawn%20Enemy
  (bind _returnvalue (Transformation|GetActorLocation))
  (bind _randomlocation (AI|Navigation|GetRandomReachablePointinRadius _returnvalue 2.5e+03 0 0))
  (if (< (Variables|Default|GetCurrentEnemies) (Variables|Default|GetMaxEnemies))
    (if (< (Math|Vector|VectorLength (- _randomlocation (Transformation|GetActorLocation (Game|GetPlayerCharacter 0)))) (Variables|Default|GetMinSpawnDistance))
      (CallFunction|SpawnEnemy)
      (else
        (bind _returnvalue_2 (Game|SpawnActorfromClass "/Game/Blueprints/Enemy/BP_Enemy_Spider.BP_Enemy_Spider_C" (Math|Transform|MakeTransform _randomlocation "0, 0, 0" "1.000000,1.000000,1.000000") "Undefined" "MultiplyWithRoot" 0 0))
        (Pawn|SpawnDefaultController _returnvalue_2)
        (bind _result (Math|Integer|IncrementInt (Variables|Default|GetCurrentEnemies))
          (:%20%20
            (Variables|Default|SetCurrentEnemies _result)
            (EventDispatchers|BindEventtoUpdateEnemyCount _returnvalue_2 (delegate Custom|NegateEnemyCountOnDeath))))))))

(event Custom|NegateEnemyCountOnDeath
  (bind _result (Math|Integer|DecrementInt (Variables|Default|GetCurrentEnemies))
    (:%20%20
      (Variables|Default|SetCurrentEnemies _result))))

(event EventBeginPlay
  (Utilities|Time|SetTimerbyEvent (delegate Custom|Spawn%20Enemy) (Variables|Default|GetSpawnInterval) true))

(fn ConstructionScript)