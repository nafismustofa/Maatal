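; BP_Enemy_Spider is a spider enemy that damages the player in melee and tracks its own health.
; Damage plays a hit montage, updates a widget health bar and triggers death at zero health.
; Attack waits briefly, sphere-traces forward for BP_Player, then applies damage on the attack montage's notify.
; Death disables movement and removes the health bar, then updates the enemy count and destroys the actor as the death montage blends out.
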(event Custom|Attack
  (bind _returnvalue (Transformation|GetActorLocation))
  (Utilities|FlowControl|Delay 0.5)
  (bind (_outhit _returnvalue_2) (Collision|SphereTraceForObjects _returnvalue (+ _returnvalue (* (Math|Vector|GetForwardVector (Transformation|GetActorRotation)) 5e+01)) 5e+01 (Utilities|Array|MakeArray "ObjectTypeQuery3") false 0 "None"))
  (if _returnvalue_2
    (bind _asbp_player (Utilities|Casting|CastToBP_Player (.HitActor (Collision|BreakHitResult _outhit))))
    (bind _notifyname (Animation|Montage|PlayMontage (Variables|Character|GetMesh) "/Game/Animations/SpiderAnimations/AM_Spider_Attack.AM_Spider_Attack")
      (:OnNotifyBegin
        (if (== _notifyname "Attack")
          (Game|Damage|ApplyDamage _asbp_player 5.0 0 0))))))

(event Custom|DeathEvent
  ;[1 1 1] Death Event
  (Variables|Default|SetIsAlive false)
  (Components|DestroyComponent (Variables|Default|GetHealthBarWidget))
  (Pawn|Components|CharacterMovement|DisableMovement (Variables|Character|GetCharacterMovement))
  (Animation|Montage|PlayMontage (Variables|Character|GetMesh) "/Game/Animations/SpiderAnimations/AM_Spider_Death.AM_Spider_Death" 1.5
    (:OnBlendOut
      (Default|CallUpdateEnemyCount)
      (Actor|DestroyActor))))

(event Game|Damage|EventAnyDamage
  (params (Damage :type Float%20%28single-precision%29) (DamageType :type Damage%20Type%20Object%20Reference) (InstigatedBy :type Controller%20Object%20Reference) (DamageCauser :type Actor%20Object%20Reference))
  ;[1 1 1] Damage Event
  (if (Variables|Default|GetIsAlive)
    (Animation|Montage|PlayMontage (Variables|Character|GetMesh) "/Game/Animations/SpiderAnimations/AM_Spider_Hit.AM_Spider_Hit"
      (:then
        (Variables|Default|SetCurrentHealth (- (Variables|Default|GetCurrentHealth) Damage))
        (bind _aswbp_enemy_health_bar (Utilities|Casting|CastToWBP_EnemyHealthBar (UserInterface|GetWidget (Variables|Default|GetHealthBarWidget))))
        (Progress|SetPercent (Variables|/Game/WidgetBlueprints/WBP_EnemyHealthBar.WBP_EnemyHealthBar_C|GetHealthBar _aswbp_enemy_health_bar) (/ (Variables|Default|GetCurrentHealth) (Variables|Default|GetMaxHealth)))
        (if (<= (Variables|Default|GetCurrentHealth) 0.0)
          (CallFunction|DeathEvent))))))

(fn ConstructionScript
  (Variables|Default|SetCurrentHealth (Variables|Default|GetMaxHealth)))